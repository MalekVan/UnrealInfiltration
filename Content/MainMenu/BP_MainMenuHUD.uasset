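; Main menu HUD that creates the menu widget on BeginPlay and hides its options and level choice panels.
; It fills the widget's key selectors from Input Settings and caches each current mapping on the widget.
; Movement keys come from the last two MoveForward and MoveRight axis entries, so mapping order matters; Interact uses its last action entry with modifiers.
; ModifyKeyBind is an empty stub whose binding never runs.
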(event Custom|ModifyKeyBind
  (params (SelectedKey :type Input%20Chord%20Structure)))

(event EventBeginPlay
  (bind _returnvalue (Class|InputSettings|GetInputSettings))
  (bind _returnvalue_2 (Class|InputSettings|GetInputSettings))
  (bind _returnvalue_3 (Class|InputSettings|GetInputSettings))
  (bind _returnvalue_4 (Class|InputSettings|GetInputSettings))
  (bind _returnvalue_5 (Class|InputSettings|GetInputSettings))
  (bind _outmappings (Class|InputSettings|GetActionMappingbyName _returnvalue_5 "Interact"))
  (bind _outmappings_2 (Class|InputSettings|GetAxisMappingbyName _returnvalue_3 "MoveForward"))
  (bind _outmappings_3 (Class|InputSettings|GetAxisMappingbyName _returnvalue_2 "MoveRight"))
  (bind _outmappings_4 (Class|InputSettings|GetAxisMappingbyName _returnvalue "MoveRight"))
  (bind _outmappings_5 (Class|InputSettings|GetAxisMappingbyName _returnvalue_4 "MoveForward"))
  (bind _returnvalue_6 (Utilities|Array|LastIndex _outmappings_3))
  (bind _returnvalue_7 (Utilities|Array|LastIndex _outmappings_2))
  (bind _returnvalue_8 (Utilities|Array|LastIndex _outmappings_5))
  (bind _returnvalue_9 (Utilities|Array|LastIndex _outmappings_4))
  (bind _returnvalue_10 (Utilities|Array|LastIndex _outmappings))
  (bind _returnvalue_11 (- _returnvalue_8 1))
  (bind _returnvalue_12 (- _returnvalue_6 1))
  (bind _output (Utilities|Array|Get(acopy) _outmappings _returnvalue_10))
  (bind _returnvalue_13 (UserInterface|CreateWidget "/Game/MainMenu/BP_MainMenuWidget.BP_MainMenuWidget_C"))
  (bind _output_get (Variables|Default|SetMainMenuWidget _returnvalue_13))
  (UserInterface|Viewport|AddtoViewport _output_get 0)
  (Widget|SetVisibility (Variables|/Game/MainMenu/BP_MainMenuWidget.BP_MainMenuWidget_C|GetOptionsPanel (Variables|Default|GetMainMenuWidget)) "Hidden")
  (Widget|SetVisibility (Variables|/Game/MainMenu/BP_MainMenuWidget.BP_MainMenuWidget_C|GetLevelChoicePanel (Variables|Default|GetMainMenuWidget)) "Hidden")
  (Utilities|FlowControl|Sequence
    (:then_0
      (Class|InputKeySelector|SetSelectedKey (Variables|/Game/MainMenu/BP_MainMenuWidget.BP_MainMenuWidget_C|GetFwdBtn (Variables|Default|GetMainMenuWidget)) (Utilities|Struct|MakeInputChord (.key (Utilities|Array|Get(acopy) _outmappings_2 _returnvalue_7)) false))
      (Variables|/Game/MainMenu/BP_MainMenuWidget.BP_MainMenuWidget_C|SetCurrentFwdKey (Variables|Default|GetMainMenuWidget) (Utilities|Array|Get(acopy) _outmappings_2 _returnvalue_7)))
    (:then_1
      (Class|InputKeySelector|SetSelectedKey (Variables|/Game/MainMenu/BP_MainMenuWidget.BP_MainMenuWidget_C|GetBwdBtn (Variables|Default|GetMainMenuWidget)) (Utilities|Struct|MakeInputChord (.key (Utilities|Array|Get(acopy) _outmappings_5 _returnvalue_11)) false))
      (Variables|/Game/MainMenu/BP_MainMenuWidget.BP_MainMenuWidget_C|SetCurrentBwdKey (Variables|Default|GetMainMenuWidget) (Utilities|Array|Get(acopy) _outmappings_5 _returnvalue_11)))
    (:then_2
      (Class|InputKeySelector|SetSelectedKey (Variables|/Game/MainMenu/BP_MainMenuWidget.BP_MainMenuWidget_C|GetLeftBtn (Variables|Default|GetMainMenuWidget)) (Utilities|Struct|MakeInputChord (.key (Utilities|Array|Get(acopy) _outmappings_4 _returnvalue_9)) false))
      (Variables|/Game/MainMenu/BP_MainMenuWidget.BP_MainMenuWidget_C|SetCurrentLeftKey (Variables|Default|GetMainMenuWidget) (Utilities|Array|Get(acopy) _outmappings_4 _returnvalue_9)))
    (:then_3
      (Class|InputKeySelector|SetSelectedKey (Variables|/Game/MainMenu/BP_MainMenuWidget.BP_MainMenuWidget_C|GetRightBtn (Variables|Default|GetMainMenuWidget)) (Utilities|Struct|MakeInputChord (.key (Utilities|Array|Get(acopy) _outmappings_3 _returnvalue_12)) false))
      (Variables|/Game/MainMenu/BP_MainMenuWidget.BP_MainMenuWidget_C|SetCurrentRightKey (Variables|Default|GetMainMenuWidget) (Utilities|Array|Get(acopy) _outmappings_3 _returnvalue_12)))
    (:then_4
      (Class|InputKeySelector|SetSelectedKey (Variables|/Game/MainMenu/BP_MainMenuWidget.BP_MainMenuWidget_C|GetInteractBtn (Variables|Default|GetMainMenuWidget)) (Utilities|Struct|MakeInputChord (.key _output) (.bshift _output) (.bctrl _output) (.balt _output) (.bcmd _output)))
      (Variables|/Game/MainMenu/BP_MainMenuWidget.BP_MainMenuWidget_C|SetCurrentInteractKey (Variables|Default|GetMainMenuWidget) (Utilities|Array|Get(acopy) _outmappings _returnvalue_10)))))

(fn ConstructionScript)