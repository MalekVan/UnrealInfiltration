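; Behavior tree service that keeps the player's position in the blackboard up to date while the player is detected.
; On each tick it reads the DetectPlayer flag and, if set, compares PosPlayer with the location of player pawn 0.
; It writes the new location only when the two differ beyond a tiny tolerance.
; A leftover debug print is never run.
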(event EventTick
  (params (OwnerActor :type Actor%20Object%20Reference) (DeltaSeconds :type Float%20%28single-precision%29))
  (bind _returnvalue (AI|GetBlackboard OwnerActor))
  (bind _returnvalue_2 (Game|Player|GetPlayerPawn 0))
  (bind _posplayer (Variables|Default|GetPosPlayer))
  (bind _returnvalue_3 (Transformation|GetActorLocation _returnvalue_2))
  (if (ScalableFloat|GetValueasBool _returnvalue (Variables|Default|GetDetectPlayer))
    (if (not (Math|Vector|Equal(Vector) (AI|Components|Blackboard|GetValueasVector _returnvalue _posplayer) _returnvalue_3 0.0001))
      (AI|Components|Blackboard|SetValueasVector _returnvalue _posplayer _returnvalue_3))))