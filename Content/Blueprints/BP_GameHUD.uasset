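; BP_GameHUD creates the player's interact prompt and pause menu widgets and handles pause toggling.
; BeginPlay enables input for player 0, adds both widgets to the viewport collapsed, and stores references to them.
; Tab switches on the menu's visibility to show or collapse it, setting game pause, mouse cursor and input mode between UI-only and game-only.
; The interact widget is only created here; nothing in this graph shows it.
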(event EventBeginPlay
  (bind _returnvalue (Game|GetPlayerController 0))
  (Utilities|FlowControl|Sequence
    (:then_0
      (Input|EnableInput _returnvalue))
    (:then_1
      (bind _returnvalue_2 (UserInterface|CreateWidget "/Game/Blueprints/BP_InteractWidget.BP_InteractWidget_C" _returnvalue))
      (UserInterface|Viewport|AddtoViewport _returnvalue_2 0)
      (Widget|SetVisibility _returnvalue_2 "Collapsed")
      (Variables|Default|SetInteractWidget _returnvalue_2))
    (:then_2
      (bind _returnvalue_3 (UserInterface|CreateWidget "/Game/Blueprints/BP_MenuWidget.BP_MenuWidget_C" _returnvalue))
      (UserInterface|Viewport|AddtoViewport _returnvalue_3 0)
      (Widget|SetVisibility _returnvalue_3 "Collapsed")
      (Variables|Default|SetPauseMenu _returnvalue_3))))

(event Input|KeyboardEvents|Tab
  (params (Key :type Key%20Structure :default "None"))
  (bind _returnvalue (Game|GetPlayerController 0))
  (bind _pausemenu (Variables|Default|GetPauseMenu))
  (:Pressed
    (switch Utilities|FlowControl|Switch|SwitchonESlateVisibility (Widget|GetVisibility (Variables|Default|GetPauseMenu))
      (:Visible
        (Widget|SetVisibility _pausemenu "Collapsed")
        (Game|SetGamePaused false)
        (Variables|/Script/Engine.PlayerController|SetbShowMouseCursor _returnvalue false)
        (Input|SetInputModeGameOnly _returnvalue))
      (:Collapsed
        (Widget|SetVisibility _pausemenu "Visible")
        (Game|SetGamePaused true)
        (Variables|/Script/Engine.PlayerController|SetbShowMouseCursor _returnvalue true)
        (Input|SetInputModeUIOnly _returnvalue (Variables|Default|GetPauseMenu) "DoNotLock")))))

(fn ConstructionScript)