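; BP_GameModeInfiltra is a game mode Blueprint containing unfinished or disconnected logic for spawning AI enemies.
; Its MakeTcheckForSpawn and SpawnIA events are empty, so neither does anything when called.
; Unwired nodes outline a loop that counts spawns up to a maximum, calling SpawnIA and rechecking after a short delay.
; Another unwired node would spawn BP_AICharacterTestP at the BpSpawner transform.
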(event Custom|MakeTcheckForSpawn
  ;[1 0 0.1133] DONE
)

(event Custom|SpawnIA
  ;[1 0 0.1133] DONE
)

(fn ConstructionScript)