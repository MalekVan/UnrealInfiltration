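; BP_Spawner is a spawn point actor for BP_GameModeInfiltra whose logic is currently disconnected, so it does nothing at runtime.
; One unwired chain would register the spawner with the game mode and trigger its spawn check.
; The other would destroy a BP_AICharacterTestP flagged GoBackToZone, decrement the game mode's enemy count and recheck spawning.
; BeginPlay, ActorBeginOverlap and the construction script are empty.
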(event EventBeginPlay
  ;[1 0.1097 0] DONE
)

(event Collision|EventActorBeginOverlap
  (params (OtherActor :type Actor%20Object%20Reference))
  ;[1 0.1097 0] DONE
)

(fn ConstructionScript)